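; Controller Blueprint that initializes the farming subsystem and spawns its grid when play begins.
; It copies its GridTextures and BPGridActor settings into the FarmingSubsystem, then calls SpawnGrid over a fixed rectangular area.
; The call supplies noise-map parameters for height, moisture and temperature, plus thresholds for sand and water and a rock percentage.
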(event EventBeginPlay
  (bind _returnvalue (Subsystems|GetFarmingSubsystem))
  (bind _array (Utilities|Array|MakeArray 2.5 5.0))
  (Variables|/Script/FarmModule.FarmingSubsystem|SetGridTextures _returnvalue (Variables|Default|GetGridTextures))
  (Variables|/Script/FarmModule.FarmingSubsystem|SetBP_GridActor _returnvalue (Variables|Default|GetBP_GridActor))
  (Class|FarmingSubsystem|SpawnGrid _returnvalue "5000.000000,-5000.000000,0.000000" "10000.000000,5000.000000,0.000000" (Utilities|Struct|MakeNoiseMapParams (Utilities|Array|MakeArray 3.5 7.0) false 0.0 true 1e+02 -1.5e+02) (Utilities|Struct|MakeNoiseMapParams _array false 0.0 true 1.0) (Utilities|Struct|MakeNoiseMapParams _array false 0.0 true 4e+01 -2e+01) 0.2 15.0 0.8 1e+01 0.02))

(fn ConstructionScript)