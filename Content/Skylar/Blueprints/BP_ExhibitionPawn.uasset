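; BP_ExhibitionPawn is an AI-controlled pawn that travels to exhibition grid cells and operates on them.
; OperateGrid stores the row and column, gets that grid actor from ExhibitionManager and issues a MoveToLocation, setting IsMoving if the request succeeds.
; When the move completes, a one-second timer clears IsMoving, and successful arrival calls the manager's OperateRange and prints the outcome.
; The manager's OnRobotEndMoving call is left unconnected.
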(event Custom|OperateGrid
  (params (Row :type Integer) (Column :type Integer))
  (Variables|Default|SetCurrRow Row)
  (Variables|Default|SetCurrCol Column)
  (bind _returnvalue (Class|ExhibitionFarmManager|GetGrid (Variables|Default|GetExhibitionManager) (Variables|Default|GetCurrRow) (Variables|Default|GetCurrCol)))
  (bind _returnvalue_2 (AI|Navigation|MovetoLocation (AI|GetAIController self) (Transformation|GetActorLocation _returnvalue) -1.0 true true false true 0))
  (Variables|Default|SetIsMoving (Utilities|Enum|Equal(Enum) _returnvalue_2 "RequestSuccessful")))

(event Custom|OnMoveEnd
  (params (RequestID :type AI%20Request%20ID%20Structure) (Result :type EPathFollowingResult%20Enum :default "Success"))
  (Utilities|Time|SetTimerbyEvent (delegate Custom|ResetIsMoving) 1.0)
  (if (Utilities|Enum|Equal(Enum) Result "Success")
    (bind _returnvalue (Class|ExhibitionFarmManager|OperateRange (Variables|Default|GetExhibitionManager) (Variables|Default|GetCurrRow) (Variables|Default|GetCurrCol)))
    (if _returnvalue
      (Development|PrintString "Operate Succeed!")
      (else
        (Development|PrintString "Operate Failed")))))

(event Custom|ResetIsMoving
  (Variables|Default|SetIsMoving false))

(event EventBeginPlay
  (EventDispatchers|BindEventtoReceiveMoveCompleted (AI|GetAIController self) (delegate Custom|OnMoveEnd)))

(fn ConstructionScript)